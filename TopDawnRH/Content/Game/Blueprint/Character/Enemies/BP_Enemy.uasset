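; BP_Enemy is an enemy Blueprint that shows damage text when hit and tracks a melee attack state.
; On BeginPlay it binds to take-any-damage, and each hit adds a widget component displaying a W_DamadgeText widget with the damage amount.
; The widget's delete event destroys that component.
; A Combat event sets the melee attack flag on change and only prints "Attack", with no attack logic.
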(event Custom|OnTakeAnyDamage_Event
  (params (DamagedActor :type Actor%20Object%20Reference) (Damage :type Float%20%28single-precision%29) (DamageType :type Damage%20Type%20Object%20Reference) (InstigatedBy :type Controller%20Object%20Reference) (DamageCauser :type Actor%20Object%20Reference))
  (bind _returnvalue (AddComponent|AddWidgetComponent false))
  (bind _returnvalue_2 (UserInterface|CreateWidget "/Game/Game/Blueprint/Widgets/W_DamadgeText.W_DamadgeText_C" 0 _returnvalue Damage))
  (UserInterface|SetWidget _returnvalue _returnvalue_2)
  (EventDispatchers|BindEventtoDelete _returnvalue_2 (delegate Custom|RemoveWidget)))

(event Custom|RemoveWidget
  (params (Parent :type Widget%20Component%20Object%20Reference))
  (Components|DestroyComponent Parent))

(event EventBeginPlay
  (EventDispatchers|BindEventtoOnTakeAnyDamage (EventDispatchers|CreateEvent :!event Custom|OnTakeAnyDamage_Event)))

(event Collision|EventActorBeginOverlap
  (params (OtherActor :type Actor%20Object%20Reference)))

(event EventTick
  (params (DeltaSeconds :type Float%20%28single-precision%29)))

(event Custom|SetMeleeAttackEnablead
  (params (IsMeleeAttack :type Boolean))
  (if (!= IsMeleeAttack (Variables|Default|GetIsMeleeAttack))
    (Variables|Default|SetIsMeleeAttack IsMeleeAttack)
    (Development|PrintString "Attack")))

(fn ConstructionScript)